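; InfinateAmmoBuff is a self-respawning runner pickup that grants the player temporary near-infinite ammo.
; On BeginPlay it waits a random Min-to-Max delay, spawns another copy ahead of the player on world X at ZValue height, then destroys itself after a further delay.
; Overlapping the ThirdPersonCharacter sets Ammo very high, then resets it to MaxAmmo after a short delay running on the pickup itself.
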(event `self.ReceiveBeginPlay`
  ;[1 1 1] Spawning
  (`KismetSystemLibrary.Delay` (`KismetMathLibrary.RandomFloatInRange` (`self.min`) (`self.max`)))
  (bind _asthird_person_character (cast `/Game/RunnerFiles/Blueprints/ThirdPersonCharacter` (`GameplayStatics.GetPlayerCharacter` 0)))
  (bind _returnvalue (`SceneComponent.K2_GetComponentToWorld` (`Actor.RootComponent` _asthird_person_character)))
  (`|SpawnActorFromClass` "InfinateAmmoBuff_C" (`KismetMathLibrary.MakeTransform` (`KismetMathLibrary.MakeVector` (+ (.x (.location _returnvalue)) 4000.0) 0.0 (`self.Z value`)) (.rotation _returnvalue) (.scale _returnvalue)) "AdjustIfPossibleButAlwaysSpawn" "OverrideRootScale" null null)
  (`KismetSystemLibrary.Delay` 10.0)
  (`self.K2_DestroyActor`))

(event `self.ReceiveActorBeginOverlap`
  (params (OtherActor :type "Actor Object Reference"))
  ;[1 1 1] Damage code
  (bind _asthird_person_character (cast `/Game/RunnerFiles/Blueprints/ThirdPersonCharacter` OtherActor))
  (set `/Game/RunnerFiles/Blueprints/ThirdPersonCharacter.Ammo` 999999.0 _asthird_person_character)
  (`KismetSystemLibrary.Delay` 5.0)
  (set `/Game/RunnerFiles/Blueprints/ThirdPersonCharacter.Ammo` (`/Game/RunnerFiles/Blueprints/ThirdPersonCharacter.Max Ammo` _asthird_person_character) _asthird_person_character))

(fn `UserConstructionScript`)