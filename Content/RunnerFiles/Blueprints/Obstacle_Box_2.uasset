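; Runner obstacle box that damages the player character on overlap and respawns copies of itself ahead along X.
; A BeginPlay timeline polls the player's Score; multiples of 1500 trigger a random delay, then a spawn at ZValue height.
; The spawning box destroys itself after a further delay.
; Overlap sets walk speed to 600, subtracts Damage from HP, prints it and calls the player controller's OnDeath without checking HP.
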(event `self.ReceiveBeginPlay`
  (`Timeline|Timeline_0`
    (:`Update`
      ;[1 1 1] Spawning
      (bind _asthird_person_character (cast `/Game/RunnerFiles/Blueprints/ThirdPersonCharacter` (`GameplayStatics.GetPlayerCharacter` 0)))
      (if (== (mod (`/Game/RunnerFiles/Blueprints/ThirdPersonCharacter.Score` _asthird_person_character) 1500) 0)
        (`KismetSystemLibrary.Delay` (`KismetMathLibrary.RandomFloatInRange` 4.0 25.0))
        (bind _returnvalue (`SceneComponent.K2_GetComponentToWorld` (`Actor.RootComponent` _asthird_person_character)))
        (`|SpawnActorFromClass` "Obstacle_Box_2_C" (`KismetMathLibrary.MakeTransform` (`KismetMathLibrary.MakeVector` (+ (.x (.location _returnvalue)) 5000.0) 0.0 (`self.Z value`)) (.rotation _returnvalue) (.scale _returnvalue)) "AdjustIfPossibleButAlwaysSpawn" "OverrideRootScale" null null)
        (`KismetSystemLibrary.Delay` 15.0)
        (`self.K2_DestroyActor`)))))

(event `self.ReceiveActorBeginOverlap`
  (params (OtherActor :type "Actor Object Reference"))
  ;[1 1 1] Damage code
  (bind _asthird_person_character (cast `/Game/RunnerFiles/Blueprints/ThirdPersonCharacter` OtherActor))
  (set `CharacterMovementComponent.MaxWalkSpeed` 600.0 (`Character.CharacterMovement` _asthird_person_character))
  (bind _output_get (set `/Game/RunnerFiles/Blueprints/ThirdPersonCharacter.HP` (`KismetMathLibrary.FTrunc` (- (`KismetMathLibrary.Conv_IntToDouble` (`/Game/RunnerFiles/Blueprints/ThirdPersonCharacter.HP` _asthird_person_character)) (`KismetMathLibrary.Conv_IntToDouble` (`self.Damage`)))) _asthird_person_character))
  (`KismetSystemLibrary.PrintString` (`KismetStringLibrary.Conv_IntToString` _output_get))
  (bind _asbp_player_controller (cast `/Game/RunnerFiles/Blueprints/BP_PlayerController` (`GameplayStatics.GetPlayerController` 0)))
  (`/Game/RunnerFiles/Blueprints/BP_PlayerController.OnDeath` _asbp_player_controller))

(fn `UserConstructionScript`)