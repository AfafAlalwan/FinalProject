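; AICharacter is an AI-controlled character that chases the player.
; BeginPlay starts Chase, which moves the pawn to the player character and repeats after a short delay on success, with no retry on failure.
; Tick sets Dead from whether HP, converted to a byte, is at or below zero, then calls DestroyActor without branching on the result.
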(event `self.ReceiveTick`
  (params (DeltaSeconds :type "Float (single-precision)"))
  (set `self.dead` (<= (`KismetMathLibrary.Conv_IntToByte` (`self.HP`)) 0))
  (`self.K2_DestroyActor` self))

(event `self.ReceiveBeginPlay`
  (`self.Chase`))

(event `Chase`
  (`|AIMoveTo` self (0.0 0.0 0.0) (`GameplayStatics.GetPlayerCharacter` 0)
    (:`OnSuccess`
      (`KismetSystemLibrary.Delay` 1.0)
      (`self.Chase`))))

(fn `UserConstructionScript`)