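; Main ground tile for a runner game that keeps the track going and awards points as the player crosses it.
; On BeginPlay it randomly decides whether to spawn a BP_SecondTile on either side, attached with relative rules so the offset follows this tile.
; When the ThirdPersonCharacter enters its box, it has ThirdPersonGameMode spawn another tile and add multiplier-scaled points, then destroys itself after a short delay.
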(event `self.ReceiveBeginPlay`
  ;[1 1 1] Attach Second Tile
  (if (`KismetMathLibrary.RandomBool`)
    (if (`KismetMathLibrary.RandomBool`)
      (set `self.SecondTilePosition` (0.0 350.0 0.0))
      (else
        (set `self.SecondTilePosition` (0.0 -350.0 0.0))))
    (bind _returnvalue (`|SpawnActorFromClass` "/Game/RunnerFiles/Blueprints/BP_SecondTile.BP_SecondTile_C" (`KismetMathLibrary.MakeTransform` (`self.SecondTilePosition`)) "Undefined" "OverrideRootScale" null null))
    (bind _output_get (set `self.SecondTile` _returnvalue))
    (`self.K2_AttachToComponent` _output_get (`self.DefaultSceneRoot`) "None" "KeepRelative" "KeepRelative" "KeepRelative" true)))

(event `self.Box.OnComponentBeginOverlap`
  (params (OverlappedComponent :type "PrimitiveComponent Object Reference") (OtherActor :type "Actor Object Reference") (OtherComp :type "PrimitiveComponent Object Reference") (OtherBodyIndex :type Integer) (bFromSweep :type Boolean) (SweepResult :type "HitResult Structure (by ref)"))
  (cast `/Game/RunnerFiles/Blueprints/ThirdPersonCharacter` OtherActor)
  (bind _asthird_person_game_mode (cast `/Game/ThirdPersonBP/Blueprints/ThirdPersonGameMode` (`GameplayStatics.GetGameMode`)))
  (`/Game/ThirdPersonBP/Blueprints/ThirdPersonGameMode.SpawnTile` _asthird_person_game_mode)
  (bind _asthird_person_game_mode_2 (cast `/Game/ThirdPersonBP/Blueprints/ThirdPersonGameMode` (`GameplayStatics.GetGameMode`)))
  (set `/Game/ThirdPersonBP/Blueprints/ThirdPersonGameMode.CurrentPoints` (+ (* (`/Game/ThirdPersonBP/Blueprints/ThirdPersonGameMode.PointsMultiplier` _asthird_person_game_mode_2) 1) (`/Game/ThirdPersonBP/Blueprints/ThirdPersonGameMode.CurrentPoints` _asthird_person_game_mode_2)) _asthird_person_game_mode_2)
  (`KismetSystemLibrary.Delay` 0.5)
  (`self.K2_DestroyActor`))

(fn `UserConstructionScript`)