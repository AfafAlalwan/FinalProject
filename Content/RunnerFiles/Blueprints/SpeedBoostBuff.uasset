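; SpeedBoostBuff is a pickup that temporarily removes the player's mesh collision and changes walk speed.
; On BeginPlay it waits a random delay, spawns its successor ahead of the player on X at a set height, then later destroys itself, forming a self-perpetuating spawn chain.
; On overlap with ThirdPersonCharacter, a timeline drives MaxWalkSpeed while mesh collision is disabled, then a delay restores collision and destroys the pickup.
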(event `self.ReceiveBeginPlay`
  ;[1 1 1] Spawning
  (`KismetSystemLibrary.Delay` (`KismetMathLibrary.RandomFloatInRange` 5.0 15.0))
  (bind _asthird_person_character (cast `/Game/RunnerFiles/Blueprints/ThirdPersonCharacter` (`GameplayStatics.GetPlayerCharacter` 0)))
  (bind _returnvalue (`SceneComponent.K2_GetComponentToWorld` (`Actor.RootComponent` _asthird_person_character)))
  (`|SpawnActorFromClass` "SpeedBoostBuff_C" (`KismetMathLibrary.MakeTransform` (`KismetMathLibrary.MakeVector` (+ (.x (.location _returnvalue)) 4000.0) 0.0 (`self.Z value`)) (.rotation _returnvalue) (.scale _returnvalue)) "AdjustIfPossibleButAlwaysSpawn" "OverrideRootScale" null null)
  (`KismetSystemLibrary.Delay` 10.0)
  (`self.K2_DestroyActor`))

(event `self.StaticMesh.OnComponentBeginOverlap`
  (params (OverlappedComponent :type "PrimitiveComponent Object Reference") (OtherActor :type "Actor Object Reference") (OtherComp :type "PrimitiveComponent Object Reference") (OtherBodyIndex :type Integer) (bFromSweep :type Boolean) (SweepResult :type "HitResult Structure (by ref)"))
  (bind _asthird_person_character (cast `/Game/RunnerFiles/Blueprints/ThirdPersonCharacter` OtherActor))
  (bind (_direction _newtrack_0) (`Timeline|Timeline_0`)
    (:`Update`
      (set `CharacterMovementComponent.MaxWalkSpeed` _newtrack_0 (`Character.CharacterMovement` _asthird_person_character))
      (bind _mesh (`Character.Mesh` _asthird_person_character))
      (`PrimitiveComponent.SetCollisionEnabled` _mesh "NoCollision")
      (`KismetSystemLibrary.Delay` 5.0)
      (`PrimitiveComponent.SetCollisionEnabled` _mesh "QueryAndPhysics")
      (`self.K2_DestroyActor`))))

(fn `UserConstructionScript`)